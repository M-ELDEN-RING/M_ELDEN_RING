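; Targeting system component that lets its owning character lock on to enemies.
; FindAllTargets sphere-traces around the owner and adds pawns tagged Enemy to a candidate list.
; LockOnToTarget sphere-sweeps along the owner camera's forward vector, picks the candidate closest to the owner and fires a lock-on event, with debug drawing left on.
; Reset functions hide the target's indicator through a message call and clear the lock.
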(fn FindAllTargets
  (bind _returnvalue (Components|GetOwner))
  (bind _returnvalue_2 (Transformation|GetActorLocation _returnvalue))
  (bind _outhits (Collision|MultiSphereTraceForObjects _returnvalue_2 _returnvalue_2 (Variables|Default|GetTraceDistance) (Utilities|Array|MakeArray "ObjectTypeQuery3") false (Utilities|Array|MakeArray (Components|GetOwner)) "None"))
  (for _array_element _outhits
    (if (Actor|ActorHasTag (.HitActor (Collision|BreakHitResult _array_element)) "Enemy")
      (Utilities|Array|AddUnique (Variables|Default|GetTargetEnemies) (.HitActor (Collision|BreakHitResult _array_element)))))
  (return (Variables|Default|GetTargetEnemies)))

(fn Initialize
  (bind _returnvalue (Components|GetOwner))
  (bind _ascharacter (Utilities|Casting|CastToCharacter _returnvalue))
  (Variables|Reference|SetCharacter _ascharacter)
  (bind _newparam (Class|BPIPlayer|Getcamera1(Message) _returnvalue))
  (Variables|Reference|SetCamera _newparam)
  (Default|CallOnResetLockedonTarget))

(fn LockontoTarget
  (bind _camera (Variables|Reference|GetCamera))
  (bind _returnvalue (Transformation|GetWorldLocation _camera))
  (Variables|Default|SetLockedOnTarget 0)
  (Utilities|IsValid (Variables|Default|GetLockedOnTarget)
    (:Is%20Not%20Valid
      (Variables|Default|SetClosestDistance (Variables|Default|GetTraceDistance))
      (bind _outhits (Collision|MultiSphereTraceForObjects _returnvalue (+ _returnvalue (* (Math|Vector|GetForwardVector _camera) (Variables|Default|GetTraceDistance))) (Variables|Default|GetRadiusToLockOn) (Utilities|Array|MakeArray "ObjectTypeQuery3") false 0 "ForDuration" true "(R=1.000000,G=0.000000,B=0.000000,A=1.000000)" "(R=0.027871,G=1.000000,B=0.066689,A=1.000000)" 2e+01))
      (for _array_element _outhits
        (if (Utilities|Array|ContainsItem (Variables|Default|GetTargetEnemies) (.HitActor (Collision|BreakHitResult _array_element)))
          (if (< (Transformation|GetDistanceTo (.HitActor (Collision|BreakHitResult _array_element)) (Components|GetOwner)) (Variables|Default|GetClosestDistance))
            (Variables|Default|SetClosestDistance (Transformation|GetDistanceTo (.HitActor (Collision|BreakHitResult _array_element)) (Components|GetOwner)))
            (Variables|Default|SetLockedOnTarget (.HitActor (Collision|BreakHitResult _array_element))))))
      (Default|CallOnLockonNewTarget)
      (return (Variables|Default|GetLockedOnTarget)))))

(fn ResetLockedonTarget
  (Utilities|IsValid (Variables|Default|GetLockedOnTarget)
    (:Is%20Valid
      (Class|BPEnemyBase|SetIndicatorVisibiility(Message) (Variables|Default|GetLockedOnTarget) false)
      (Variables|Default|SetLockedOnTarget 0))))

(fn ResetLockedonTarget
  (Utilities|IsValid (Variables|Default|GetLockedOnTarget)
    (:Is%20Valid
      (Class|BPEnemyBase|SetIndicatorVisibiility(Message) (Variables|Default|GetLockedOnTarget) false)
      (Variables|Default|SetLockedOnTarget 0)
      (Default|CallOnResetLockedonTarget))))